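; Game mode for AnotherWorldStreet that handles procedural map setup, game start and game end.
; InitializeGame spawns BP_MapGeneratorBase, shows a loading screen and runs a genetic algorithm, whose completion fires the init-end delegate with Result false and a start location.
; OnInitializeEnded, only on a true Result, teleports the player, starts a looping elapsed-time timer and shows the in-game HUD.
; FinishGame stops the timer, broadcasts elapsed time and slows global time.
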(event Custom|CustomEvent
  (params (StartLocation :type Vector) (TotalElapsedTime :type Float%20%28single-precision%29))
  ;[1 0.8958 0.9598 1 24] 맵 생성기를 스폰하고, 로딩 UI 초기화 및 GA를 돌린다. / 종료 시점의 이벤트 또한 바인딩한다
  (Default|CallOnInitializeEndDelegate false StartLocation)
  (Development|PrintString (Utilities|String|Append "Total Elapsed Time : " (Utilities|String|ToString(Float) TotalElapsedTime)) true true "(R=1.000000,G=0.953935,B=0.000000,A=1.000000)" 5e+04))

(event EventInitializeGame
  ;[1 0.8958 0.9598 1 24] 맵 생성기를 스폰하고, 로딩 UI 초기화 및 GA를 돌린다. / 종료 시점의 이벤트 또한 바인딩한다
  (bind _mapgeneratorref (CallFunction|SpawnMapGenerator))
  (Utilities|IsValid _mapgeneratorref
    (:Is%20Valid
      (Utilities|FlowControl|Sequence
        (:then_0
          (bind _returnvalue (UserInterface|CreateWidget "/Game/UI/WB_LoadingScreen.WB_LoadingScreen_C" (Game|GetPlayerController 0))) ; 로딩 UI 생성
          (UserInterface|Viewport|AddtoViewport _returnvalue 0)
          (Default|InitLoadingScreen _returnvalue _mapgeneratorref))
        (:then_1
          (EventDispatchers|BindEventtoOnGAEndProcess _mapgeneratorref (delegate Custom|CustomEvent)) ; GA 종료시점 바인딩
          (Class|MapGeneratorBase|RunGeneticAlgorithm _mapgeneratorref) ; GA 돌리기
        )))))

(event EventOnInitializeEnded
  (params (Result :type Boolean) (StartLocation :type Vector :default "0, 0, 0"))
  ;[1 1 1] 게임시작
  (if Result
    (Transformation|SetActorLocation (Game|GetPlayerCharacter 0) StartLocation false true)
    (Class|AnotherWorldStreetGameModeBase|StartGame)))

(event EventStartGame
  ;[1 1 1] 게임 타이머를 초기화한다
  (bind _returnvalue (CallFunction|StartGameTimer))
  (Variables|Non-Edit|SetGameTimerHandle _returnvalue)
  (bind _returnvalue_2 (UserInterface|CreateWidget "/Game/UI/WB_Ingame.WB_Ingame_C" (Game|GetPlayerController 0)))
  (UserInterface|Viewport|AddtoViewport _returnvalue_2 0))

(event EventFinishGame
  ;[1 1 1] 게임을 끝낸다
  (Utilities|Time|ClearandInvalidateTimerbyHandle (Variables|Non-Edit|GetGameTimerHandle))
  (Default|CallOnGameFinishedDelegate (CallFunction|GetGameElapsedTime))
  (Utilities|Time|SetGlobalTimeDilation 0.1))

(fn ConstructionScript)

(fn SpawnMapGenerator
  (bind _returnvalue (Game|SpawnActorfromClass "/Game/System/Blueprint/BP_MapGeneratorBase.BP_MapGeneratorBase_C" (Math|Transform|MakeTransform "0, 0, 0" "0, 0, 0" "1.000000,1.000000,1.000000") "Undefined" "MultiplyWithRoot" self 0))
  (return _returnvalue))

(fn StartGameTimer
  (bind _returnvalue (Utilities|Time|SetTimerbyFunctionName self "UpdateGameTimer" (Variables|Settings|GetTimerInterval) true))
  (return _returnvalue))

(fn UpdateGameTimer
  (Variables|Non-Edit|SetElapsedTime (+ (Variables|Non-Edit|GetElapsedTime) (Variables|Settings|GetTimerInterval)))
  (return))

(fn GetGameElapsedTime
  (return (Variables|Non-Edit|GetElapsedTime)))