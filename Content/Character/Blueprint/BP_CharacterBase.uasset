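; Base character Blueprint for a third-person player with movement, look, jump, sprint, aim and wand attack through Enhanced Input.
; Sprint doubles and restores walk speed behind a state flag.
; Aiming reattaches the camera between two spring arms, eases it across with MoveComponentTo, and switches rotation between movement-facing and controller yaw.
; Firing works only while aiming, playing a wand montage and blocking repeats for its duration.
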(event Custom|InitInput
  ;[1 0.5782 0.7204 1 50] Input
  (Input|AddMappingContext (PlayerController|LocalPlayerSubsystems|GetEnhancedInputLocalPlayerSubsystem (Game|GetPlayerController 0)) (Variables|Input|GetIMC_Default) 0 "(bIgnoreAllPressedKeysUntilRelease=True,bForceImmediately=False)"))

(event Custom|TryFire
  ;[1 0.5782 0.7204 1 50] Input
  ;;[1 1 1] 코멘트
  (if (and (Variables|Default|GetbIsAiming) (not (Variables|Default|GetbIsAttacking)))
    (Variables|Default|SetbIsAttacking true)
    (bind _returnvalue (Animation|PlayAnimMontage "/Game/Character/Animation/Montage/AM_WandAttack_1.AM_WandAttack_1" 1.0 "None"))
    (Utilities|FlowControl|Delay _returnvalue)
    (Variables|Default|SetbIsAttacking false)))

(event Custom|StopAim
  ;[1 0.5782 0.7204 1 50] Input
  ;;[1 1 1] 코멘트
  (Variables|Default|SetbIsAiming false)
  (Transformation|AttachComponentToComponent (Variables|Default|GetCamera) (Variables|Default|GetSpringArm) "None" "KeepWorld" "KeepWorld" "KeepWorld" true)
  (Components|MoveComponentTo (Variables|Default|GetCamera) "0, 0, 0" "0, 0, 0" true true 0.2 false))

(event Custom|Aim
  (bind _camera (Variables|Default|GetCamera))
  ;[1 0.5782 0.7204 1 50] Input
  ;;[1 1 1] 코멘트
  (Variables|Default|SetbIsAiming true)
  (Transformation|AttachComponentToComponent _camera (Variables|Default|GetAimSpringArm) "None" "KeepWorld" "KeepWorld" "KeepWorld" true)
  (Components|MoveComponentTo _camera "0, 0, 0" "0, 0, 0" true true 0.2 false))

(event Input|EnhancedActionEvents|EnhancedInputActionIA_Look
  (params (ActionValue :type Vector%202D%20Structure) (ElapsedSeconds :type Float%20%28double-precision%29) (TriggeredSeconds :type Float%20%28double-precision%29) (InputAction :type Input%20Action%20Object%20Reference :default "/Game/Character/Input/IA_Look.IA_Look"))
  (bind (_x _y) (Math|Vector2D|BreakVector2D ActionValue))
  ;[1 0.5782 0.7204 1 50] Input
  (:Triggered
    (Pawn|Input|AddControllerYawInput _x)
    (Pawn|Input|AddControllerPitchInput _y)))

(event Input|EnhancedActionEvents|EnhancedInputActionIA_Move
  (params (ActionValue :type Vector%202D%20Structure) (ElapsedSeconds :type Float%20%28double-precision%29) (TriggeredSeconds :type Float%20%28double-precision%29) (InputAction :type Input%20Action%20Object%20Reference :default "/Game/Character/Input/IA_Move.IA_Move"))
  (bind _returnvalue (Pawn|GetControlRotation :!class /Script/Engine.Pawn))
  ;[1 0.5782 0.7204 1 50] Input
  (:Triggered
    (Pawn|Input|AddMovementInput (Math|Vector|GetRightVector (Math|Rotator|MakeRotator (.roll _returnvalue) 0.0 (.yaw _returnvalue))) (.x ActionValue) false)
    (Pawn|Input|AddMovementInput (Math|Vector|GetForwardVector (Math|Rotator|MakeRotator 0.0 0.0 (.yaw (Pawn|GetControlRotation :!class /Script/Engine.Pawn)))) (.y ActionValue) false)))

(event Input|EnhancedActionEvents|EnhancedInputActionIA_Jump
  (params (ActionValue :type Boolean) (ElapsedSeconds :type Float%20%28double-precision%29) (TriggeredSeconds :type Float%20%28double-precision%29) (InputAction :type Input%20Action%20Object%20Reference :default "/Game/Character/Input/IA_Jump.IA_Jump"))
  ;[1 0.5782 0.7204 1 50] Input
  (:Triggered
    (Character|Jump)))

(event Input|EnhancedActionEvents|EnhancedInputActionIA_Sprint
  (params (ActionValue :type Boolean) (ElapsedSeconds :type Float%20%28double-precision%29) (TriggeredSeconds :type Float%20%28double-precision%29) (InputAction :type Input%20Action%20Object%20Reference :default "/Game/Character/Input/IA_Sprint.IA_Sprint"))
  (bind _charactermovement (Variables|Character|GetCharacterMovement))
  ;[1 0.5782 0.7204 1 50] Input
  (:Triggered
    (if (not (Variables|Default|GetbIsSprinting))
      (Variables|/Script/Engine.CharacterMovementComponent|SetMaxWalkSpeed _charactermovement (* (Variables|/Script/Engine.CharacterMovementComponent|GetMaxWalkSpeed _charactermovement) 2.0))
      (Variables|Default|SetbIsSprinting true))))

(event Input|EnhancedActionEvents|EnhancedInputActionIA_Aim
  (params (ActionValue :type Boolean) (ElapsedSeconds :type Float%20%28double-precision%29) (TriggeredSeconds :type Float%20%28double-precision%29) (InputAction :type Input%20Action%20Object%20Reference :default "/Game/Character/Input/IA_Aim.IA_Aim"))
  ;[1 0.5782 0.7204 1 50] Input
  (:Triggered
    (Variables|/Script/Engine.CharacterMovementComponent|SetbOrientRotationToMovement (Variables|Character|GetCharacterMovement) false)
    (Variables|Default|SetbUseControllerRotationYaw true)
    (CallFunction|Aim)))

(event Input|EnhancedActionEvents|EnhancedInputActionIA_Fire
  (params (ActionValue :type Boolean) (ElapsedSeconds :type Float%20%28double-precision%29) (TriggeredSeconds :type Float%20%28double-precision%29) (InputAction :type Input%20Action%20Object%20Reference :default "/Game/Character/Input/IA_Fire.IA_Fire"))
  ;[1 0.5782 0.7204 1 50] Input
  (:Triggered
    (CallFunction|TryFire)))

(event Input|EnhancedActionEvents|EnhancedInputActionIA_StopAim
  (params (ActionValue :type Boolean) (ElapsedSeconds :type Float%20%28double-precision%29) (TriggeredSeconds :type Float%20%28double-precision%29) (InputAction :type Input%20Action%20Object%20Reference :default "/Game/Character/Input/IA_StopAim.IA_StopAim"))
  ;[1 0.5782 0.7204 1 50] Input
  (:Triggered
    (Variables|/Script/Engine.CharacterMovementComponent|SetbOrientRotationToMovement (Variables|Character|GetCharacterMovement) true)
    (Variables|Default|SetbUseControllerRotationYaw false)
    (CallFunction|StopAim)))

(event Input|EnhancedActionEvents|EnhancedInputActionIA_StopSprint
  (params (ActionValue :type Boolean) (ElapsedSeconds :type Float%20%28double-precision%29) (TriggeredSeconds :type Float%20%28double-precision%29) (InputAction :type Input%20Action%20Object%20Reference :default "/Game/Character/Input/IA_StopSprint.IA_StopSprint"))
  (bind _charactermovement (Variables|Character|GetCharacterMovement))
  ;[1 0.5782 0.7204 1 50] Input
  (:Triggered
    (if (Variables|Default|GetbIsSprinting)
      (Variables|/Script/Engine.CharacterMovementComponent|SetMaxWalkSpeed _charactermovement (* (Variables|/Script/Engine.CharacterMovementComponent|GetMaxWalkSpeed _charactermovement) 0.5))
      (Variables|Default|SetbIsSprinting false))))

(event EventBeginPlay
  ;[1 0.9124 0] Initialize
  (CallFunction|InitInput))

(fn ConstructionScript)