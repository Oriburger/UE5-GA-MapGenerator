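; BP_CalculatedSpline is a spline actor that tiles a static mesh along its path at construction time, with no active gameplay logic.
; The construction script divides spline length by MeshLength, truncating any remainder, and adds one spline mesh component per whole segment.
; Each segment takes local positions and tangents clamped to MeshLength, using the configurable mesh and forward axis.
; It also draws a debug box from the mesh's untransformed bounds.
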(event EventBeginPlay)

(event Collision|EventActorBeginOverlap
  (params (OtherActor :type Actor%20Object%20Reference)))

(event EventTick
  (params (DeltaSeconds :type Float%20%28single-precision%29)))

(fn ConstructionScript
  (bind _spline (Variables|Default|GetSpline))
  (bind _meshlength (Variables|Default|GetMeshLength))
  (bind _new_mesh (Variables|Default|GetNew%20Mesh))
  (bind _spline_2 (Variables|Default|GetSpline))
  (bind _meshlength_2 (Variables|Default|GetMeshLength))
  (bind _returnvalue (StaticMesh|GetBoundingBox _new_mesh))
  (bind (_min _max) (Utilities|Struct|BreakBox _returnvalue))
  (for _index (range 0 (- (Math|Float|Truncate (/ (Spline|GetSplineLength (Variables|Default|GetSpline)) _meshlength)) 1))
    (bind _returnvalue_2 (AddComponent|AddSplineMeshComponent false))
    (SplineMesh|SetForwardAxis _returnvalue_2 (Variables|Default|GetIn%20Forward%20Axis) true)
    (SplineMesh|SetStartandEnd _returnvalue_2 (Spline|GetLocationatDistanceAlongSpline _spline_2 (* _index _meshlength) "Local") (Math|Vector|ClampVectorSize (Spline|GetTangentatDistanceAlongSpline _spline_2 (* _index _meshlength) "Local") 1.0 _meshlength_2) (Spline|GetLocationatDistanceAlongSpline _spline (* (+ _index 1) _meshlength) "Local") (Math|Vector|ClampVectorSize (Spline|GetTangentatDistanceAlongSpline _spline (* (+ _index 1) _meshlength) "Local") 1.0 _meshlength_2) true :!class /Script/Engine.SplineMeshComponent)
    (Components|StaticMesh|SetStaticMesh _returnvalue_2 _new_mesh)
    (Rendering|Debug|DrawDebugBox :Center (/ (+ _min _max) "2.000000,2.000000,2.000000") :Extent (/ (- _min _max) "2.000000,2.000000,2.000000"))))