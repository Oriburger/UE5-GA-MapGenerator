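; Spline actor that lays a configurable static mesh along its spline, with all logic in the Construction Script and an empty Event Graph.
; The script applies the closed-loop setting, then adds one Spline Mesh component per segment with the chosen mesh and forward axis.
; Each segment takes its ends and tangents from neighboring points in local space.
; A fixed 270-degree roll is set on each component and each segment's start point.
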(event EventBeginPlay)

(event Collision|EventActorBeginOverlap
  (params (OtherActor :type Actor%20Object%20Reference)))

(event EventTick
  (params (DeltaSeconds :type Float%20%28single-precision%29)))

(fn ConstructionScript
  (bind _returnvalue (Math|Rotator|MakeRotator 2.7e+02 0.0 0.0))
  (bind _spline (Variables|Default|GetSpline))
  (Utilities|FlowControl|Sequence
    (:then_0
      (Spline|SetClosedLoop (Variables|Default|GetSpline) (Variables|Default|GetIn%20Closed%20Loop) true))
    (:then_1
      (for _index (range 0 (- (Class|SplineComponent|GetNumberOfSplineSegments (Variables|Default|GetSpline)) 1))
        (bind _returnvalue_2 (AddComponent|AddSplineMeshComponent false (Math|Transform|MakeTransform "0, 0, 0" _returnvalue)))
        (SplineMesh|SetForwardAxis _returnvalue_2 (Variables|Default|GetIn%20Forward%20Axis) true)
        (Spline|SetRotationatSplinePoint (Variables|Default|GetSpline) _index _returnvalue "Local" true)
        (SplineMesh|SetStartandEnd _returnvalue_2 (.Location (Spline|GetLocationandTangentatSplinePoint _spline _index "Local")) (.Tangent (Spline|GetLocationandTangentatSplinePoint _spline _index "Local")) (.Location (Spline|GetLocationandTangentatSplinePoint _spline (+ _index 1) "Local")) (.Tangent (Spline|GetLocationandTangentatSplinePoint _spline (+ _index 1) "Local")) true :!class /Script/Engine.SplineMeshComponent)
        (Components|StaticMesh|SetStaticMesh _returnvalue_2 (Variables|Default|GetNew%20Mesh))))))