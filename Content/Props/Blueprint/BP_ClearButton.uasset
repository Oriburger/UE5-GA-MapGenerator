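; BP_ClearButton is a floor-button prop that ends the game when an actor tagged "Player" overlaps its Box.
; On that overlap it lowers the Button component, spawns a particle emitter just above the actor and calls FinishGame on BP_AnotherWorldStreetGameMode.
; A DoOnce runs before the tag check, so the first overlap by any actor consumes the trigger, even if it is not the player.
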(event OnComponentBeginOverlap(Box)
  (params (OverlappedComponent :type Primitive%20Component%20Object%20Reference) (OtherActor :type Actor%20Object%20Reference) (OtherComp :type Primitive%20Component%20Object%20Reference) (OtherBodyIndex :type Integer) (bFromSweep :type Boolean) (SweepResult :type Hit%20Result%20Structure%20%28by%20ref%29))
  (bind _returnvalue (Transformation|GetActorLocation))
  (Utilities|FlowControl|DoOnce false
    (:Completed
      (if (Actor|ActorHasTag OtherActor "Player")
        (Transformation|SetRelativeLocation (Variables|Default|GetButton) "0.000000,0.000000,-10.000000" false false)
        (Effects|SpawnEmitteratLocation "/Engine/Tutorial/SubEditors/TutorialAssets/TutorialParticleSystem.TutorialParticleSystem" (Math|Vector|MakeVector (.x _returnvalue) (.y _returnvalue) (+ (.z _returnvalue) 1e+01)))
        (bind _asbp_another_world_street_game_mode (Utilities|Casting|CastToBP_AnotherWorldStreetGameMode (Game|GetGameMode)))
        (Class|AnotherWorldStreetGameModeBase|FinishGame _asbp_another_world_street_game_mode)))))

(event EventBeginPlay)

(event Collision|EventActorBeginOverlap
  (params (OtherActor :type Actor%20Object%20Reference)))

(event EventTick
  (params (DeltaSeconds :type Float%20%28single-precision%29)))

(fn ConstructionScript)