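; BP_MapGeneratorBase coordinates initial map generation and map visualization through components.
; CreateInitialMap runs one of two interchangeable generator components (DH or YH, hardwired to DH) and passes its last result to SetInitialPopulation as a one-map population.
; Visualize forwards MapInfo to BPMapVisualizerComponent.
; BeginPlay can jump straight into generation, but a constant false branch disables that path.
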(event EventCreateInitialMap
  (bind _bp_initialmapgeneratorcomponent_yh (Variables|Default|GetBP_InitialMapGeneratorComponent_YH))
  (bind _bp_initialmapgeneratorcomponent_dh (Variables|Default|GetBP_InitialMapGeneratorComponent_DH))
  (bind _returnvalue (select true _bp_initialmapgeneratorcomponent_dh _bp_initialmapgeneratorcomponent_yh))
  ;[1 1 1] 초기 맵 생성
  (Class|InitialMapGeneratorComponent|Generate _returnvalue) ; 유호, 대현형이 구현해야하는 것
  (Class|MapGeneratorBase|SetInitialPopulation (Utilities|Array|MakeArray (Class|InitialMapGeneratorComponent|GetLastResult _returnvalue))) ; 지우면 안되빈다
)

(event EventVisualize
  (params (MapInfo :type Map%20Info%20Struct%20Structure))
  ;[1 1 1] 시각화 과정
  (Class|MapVisualizerComponent|Visualize (Variables|Default|GetBP_MapVisualizerComponent) MapInfo) ; 창우리 -> 이 함수 만들어주세요
)

(event EventBeginPlay
  (bind _bp_initialmapgeneratorcomponent_yh (Variables|Default|GetBP_InitialMapGeneratorComponent_YH))
  (bind _bp_initialmapgeneratorcomponent_dh (Variables|Default|GetBP_InitialMapGeneratorComponent_DH))
  (bind _returnvalue (select true _bp_initialmapgeneratorcomponent_dh _bp_initialmapgeneratorcomponent_yh))
  ;[1 1 1] 시각화 과정
  (if false ; '딸깍'만 하세요
    ;[1 1 1] 초기 맵 생성
    (Class|InitialMapGeneratorComponent|Generate _returnvalue) ; 유호, 대현형이 구현해야하는 것
    (Class|MapGeneratorBase|SetInitialPopulation (Utilities|Array|MakeArray (Class|InitialMapGeneratorComponent|GetLastResult _returnvalue))) ; 지우면 안되빈다
  ))

(fn ConstructionScript)