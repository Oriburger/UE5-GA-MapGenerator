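; Map generator component that builds an initial platform path from the owning BP_MapGeneratorBase's start to end location.
; Generate steps along that line at player max speed, placing a platform every PlatformIntervalSecond, plus one at second 1.
; Random X/Z offsets add variation, while climbs exceeding MaximumJumpHeight are capped relative to the previous platform.
; It records the list in LastGenerateResultList and spawns debug meshes; the SetPerlinVector noise helper is not called here.
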(event EventGenerate
  (bind _returnvalue (Game|GetPlayerCharacter 0))
  (bind _returnvalue_2 (Math|Random|RandomFloat))
  (bind _platformlist (Variables|Default|GetPlatformList))
  (bind _maximumjumpheight (Variables|Default|GetMaximumJumpHeight))
  (bind _noiseweight (Variables|Default|GetNoiseWeight))
  (bind _returnvalue_3 (Utilities|Array|LastIndex _platformlist))
  (bind _returnvalue_4 (* _returnvalue_2 _noiseweight))
  (bind _charactermovement (Variables|/Script/Engine.Character|GetCharacterMovement _returnvalue))
  (bind _returnvalue_5 (Class|MovementComponent|GetMaxSpeed _charactermovement))
  (bind _output (Utilities|Array|Get(acopy) _platformlist _returnvalue_3))
  (bind _platformtransform (Utilities|Struct|BreakPlatformInfoStruct _output))
  (bind _z (Math|Vector|BreakVector (.location _platformtransform)))
  ;[0.9667 0.4177 1 1 33] 맵 생성 알고리즘 2 _ 권대현
  ;;[1 1 1] Get Reference
  (|CallParentFunction)
  (bind _asbp_map_generator_base (Utilities|Casting|CastToBP_MapGeneratorBase (Components|GetOwner)))
  (Utilities|Array|Add _platformlist (Utilities|Struct|MakePlatformInfoStruct "/Game/Asset/Platformer/Meshes/Pl_8m_Platform.Pl_8m_Platform" (Math|Conversions|ToTransform(Vector) (Variables|/Script/AnotherWorldStreet.MapGeneratorBase|GetStartLocation _asbp_map_generator_base))))
  ;[1 1 1] 메시 생성(디버그)
  (bind _returnvalue_6 (Game|AddComponentbyClass _asbp_map_generator_base "/Script/Engine.StaticMeshComponent" false (Math|Conversions|ToTransform(Vector) (Variables|/Script/AnotherWorldStreet.MapGeneratorBase|GetStartLocation _asbp_map_generator_base))))
  (Components|StaticMesh|SetStaticMesh _returnvalue_6 "/Game/Asset/Platformer/Meshes/Pl_8m_Platform_rnd.Pl_8m_Platform_rnd")
  (for _index (range 1 (- (Math|Float|Ceil (/ (Math|Vector|Distance(Vector) (Variables|/Script/AnotherWorldStreet.MapGeneratorBase|GetStartLocation _asbp_map_generator_base) (Variables|/Script/AnotherWorldStreet.MapGeneratorBase|GetEndLocation _asbp_map_generator_base)) _returnvalue_5)) (Variables|Default|GetPlatformIntervalSecond)))
    (Class|KismetMathLibrary|SeedRandomStream (Math|Random|MakeRandomStream (Math|Random|RandomInteger 999)))
    (if (== (Math|Integer|%(Integer) _index (Variables|Default|GetPlatformIntervalSecond)) 0)
      (if (> (- (.Z (Math|Vector|BreakVector (Math|Interpolation|VInterptoConstant (Variables|/Script/AnotherWorldStreet.MapGeneratorBase|GetStartLocation _asbp_map_generator_base) (Variables|/Script/AnotherWorldStreet.MapGeneratorBase|GetEndLocation _asbp_map_generator_base) (Math|Conversions|ToFloat(Integer) _index) _returnvalue_5))) _z) _maximumjumpheight) :!label _label
        (Utilities|Array|Add _platformlist (Utilities|Struct|MakePlatformInfoStruct "/Game/Asset/Platformer/Meshes/Pl_8m_Platform.Pl_8m_Platform" (Math|Transform|MakeTransform (Math|Vector|MakeVector (+ (.X (Math|Vector|BreakVector (Math|Interpolation|VInterptoConstant (Variables|/Script/AnotherWorldStreet.MapGeneratorBase|GetStartLocation _asbp_map_generator_base) (Variables|/Script/AnotherWorldStreet.MapGeneratorBase|GetEndLocation _asbp_map_generator_base) (Math|Conversions|ToFloat(Integer) _index) _returnvalue_5))) (* _returnvalue_4 2.0)) (.Y (Math|Vector|BreakVector (Math|Interpolation|VInterptoConstant (Variables|/Script/AnotherWorldStreet.MapGeneratorBase|GetStartLocation _asbp_map_generator_base) (Variables|/Script/AnotherWorldStreet.MapGeneratorBase|GetEndLocation _asbp_map_generator_base) (Math|Conversions|ToFloat(Integer) _index) _returnvalue_5))) (+ _maximumjumpheight _z)))))
        (Development|PrintString (Utilities|String|ToString(Transform) (Math|Transform|MakeTransform (Math|Vector|MakeVector (+ (.X (Math|Vector|BreakVector (Math|Interpolation|VInterptoConstant (Variables|/Script/AnotherWorldStreet.MapGeneratorBase|GetStartLocation _asbp_map_generator_base) (Variables|/Script/AnotherWorldStreet.MapGeneratorBase|GetEndLocation _asbp_map_generator_base) (Math|Conversions|ToFloat(Integer) _index) _returnvalue_5))) (* _returnvalue_4 2.0)) (.Y (Math|Vector|BreakVector (Math|Interpolation|VInterptoConstant (Variables|/Script/AnotherWorldStreet.MapGeneratorBase|GetStartLocation _asbp_map_generator_base) (Variables|/Script/AnotherWorldStreet.MapGeneratorBase|GetEndLocation _asbp_map_generator_base) (Math|Conversions|ToFloat(Integer) _index) _returnvalue_5))) (+ _maximumjumpheight _z)))))
        ;[1 1 1] 메시 생성(디버그)
        (bind _returnvalue_7 (Game|AddComponentbyClass _asbp_map_generator_base "/Script/Engine.StaticMeshComponent" false (Math|Transform|MakeTransform (Math|Vector|MakeVector (+ (.X (Math|Vector|BreakVector (Math|Interpolation|VInterptoConstant (Variables|/Script/AnotherWorldStreet.MapGeneratorBase|GetStartLocation _asbp_map_generator_base) (Variables|/Script/AnotherWorldStreet.MapGeneratorBase|GetEndLocation _asbp_map_generator_base) (Math|Conversions|ToFloat(Integer) _index) _returnvalue_5))) (* _returnvalue_4 2.0)) (.Y (Math|Vector|BreakVector (Math|Interpolation|VInterptoConstant (Variables|/Script/AnotherWorldStreet.MapGeneratorBase|GetStartLocation _asbp_map_generator_base) (Variables|/Script/AnotherWorldStreet.MapGeneratorBase|GetEndLocation _asbp_map_generator_base) (Math|Conversions|ToFloat(Integer) _index) _returnvalue_5))) (+ _maximumjumpheight _z)))))
        (Components|StaticMesh|SetStaticMesh _returnvalue_7 "/Game/Asset/Platformer/Meshes/Pl_8m_Platform.Pl_8m_Platform")
        (else
          (Utilities|Array|Add _platformlist (Utilities|Struct|MakePlatformInfoStruct "/Game/Asset/Platformer/Meshes/Pl_8m_Platform.Pl_8m_Platform" (Math|Transform|MakeTransform (Math|Vector|MakeVector (+ (.X (Math|Vector|BreakVector (Math|Interpolation|VInterptoConstant (Variables|/Script/AnotherWorldStreet.MapGeneratorBase|GetStartLocation _asbp_map_generator_base) (Variables|/Script/AnotherWorldStreet.MapGeneratorBase|GetEndLocation _asbp_map_generator_base) (Math|Conversions|ToFloat(Integer) _index) _returnvalue_5))) (* _returnvalue_4 2.0)) (.Y (Math|Vector|BreakVector (Math|Interpolation|VInterptoConstant (Variables|/Script/AnotherWorldStreet.MapGeneratorBase|GetStartLocation _asbp_map_generator_base) (Variables|/Script/AnotherWorldStreet.MapGeneratorBase|GetEndLocation _asbp_map_generator_base) (Math|Conversions|ToFloat(Integer) _index) _returnvalue_5))) (+ (.Z (Math|Vector|BreakVector (Math|Interpolation|VInterptoConstant (Variables|/Script/AnotherWorldStreet.MapGeneratorBase|GetStartLocation _asbp_map_generator_base) (Variables|/Script/AnotherWorldStreet.MapGeneratorBase|GetEndLocation _asbp_map_generator_base) (Math|Conversions|ToFloat(Integer) _index) _returnvalue_5))) (/ _returnvalue_4 2.0))))))
          (Development|PrintString (Utilities|String|ToString(Transform) (Math|Transform|MakeTransform (Math|Vector|MakeVector (+ (.X (Math|Vector|BreakVector (Math|Interpolation|VInterptoConstant (Variables|/Script/AnotherWorldStreet.MapGeneratorBase|GetStartLocation _asbp_map_generator_base) (Variables|/Script/AnotherWorldStreet.MapGeneratorBase|GetEndLocation _asbp_map_generator_base) (Math|Conversions|ToFloat(Integer) _index) _returnvalue_5))) (* _returnvalue_4 2.0)) (.Y (Math|Vector|BreakVector (Math|Interpolation|VInterptoConstant (Variables|/Script/AnotherWorldStreet.MapGeneratorBase|GetStartLocation _asbp_map_generator_base) (Variables|/Script/AnotherWorldStreet.MapGeneratorBase|GetEndLocation _asbp_map_generator_base) (Math|Conversions|ToFloat(Integer) _index) _returnvalue_5))) (+ (.Z (Math|Vector|BreakVector (Math|Interpolation|VInterptoConstant (Variables|/Script/AnotherWorldStreet.MapGeneratorBase|GetStartLocation _asbp_map_generator_base) (Variables|/Script/AnotherWorldStreet.MapGeneratorBase|GetEndLocation _asbp_map_generator_base) (Math|Conversions|ToFloat(Integer) _index) _returnvalue_5))) (/ _returnvalue_4 2.0))))))
          ;[1 1 1] 메시 생성(디버그)
          (bind _returnvalue_8 (Game|AddComponentbyClass _asbp_map_generator_base "/Script/Engine.StaticMeshComponent" false (Math|Transform|MakeTransform (Math|Vector|MakeVector (+ (.X (Math|Vector|BreakVector (Math|Interpolation|VInterptoConstant (Variables|/Script/AnotherWorldStreet.MapGeneratorBase|GetStartLocation _asbp_map_generator_base) (Variables|/Script/AnotherWorldStreet.MapGeneratorBase|GetEndLocation _asbp_map_generator_base) (Math|Conversions|ToFloat(Integer) _index) _returnvalue_5))) (* _returnvalue_4 2.0)) (.Y (Math|Vector|BreakVector (Math|Interpolation|VInterptoConstant (Variables|/Script/AnotherWorldStreet.MapGeneratorBase|GetStartLocation _asbp_map_generator_base) (Variables|/Script/AnotherWorldStreet.MapGeneratorBase|GetEndLocation _asbp_map_generator_base) (Math|Conversions|ToFloat(Integer) _index) _returnvalue_5))) (+ (.Z (Math|Vector|BreakVector (Math|Interpolation|VInterptoConstant (Variables|/Script/AnotherWorldStreet.MapGeneratorBase|GetStartLocation _asbp_map_generator_base) (Variables|/Script/AnotherWorldStreet.MapGeneratorBase|GetEndLocation _asbp_map_generator_base) (Math|Conversions|ToFloat(Integer) _index) _returnvalue_5))) (/ _returnvalue_4 2.0))))))
          (Components|StaticMesh|SetStaticMesh _returnvalue_8 "/Game/Asset/Platformer/Meshes/Pl_8m_Platform.Pl_8m_Platform")))
      (elif (== _index 1)
        (goto _label))))
  (Utilities|Array|Add _platformlist (Utilities|Struct|MakePlatformInfoStruct "/Game/Asset/Platformer/Meshes/Pl_8m_Platform.Pl_8m_Platform" (Math|Conversions|ToTransform(Vector) (Variables|/Script/AnotherWorldStreet.MapGeneratorBase|GetEndLocation _asbp_map_generator_base))))
  ;[1 1 1] 메시 생성(디버그)
  (bind _returnvalue_9 (Game|AddComponentbyClass _asbp_map_generator_base "/Script/Engine.StaticMeshComponent" false (Math|Conversions|ToTransform(Vector) (Variables|/Script/AnotherWorldStreet.MapGeneratorBase|GetEndLocation _asbp_map_generator_base))))
  (Components|StaticMesh|SetStaticMesh _returnvalue_9 "/Game/Asset/Platformer/Meshes/Pl_8m_Platform_rnd.Pl_8m_Platform_rnd")
  (Utilities|Array|Add (Variables|Default|GetLastGenerateResultList) (Utilities|Struct|MakeMapInfoStruct _platformlist 0 0.0)))

(fn SetPerlinVector
  (params (Vector :type Vector) (FastNoiseWrapper :type Fast%20Noise%20Wrapper%20Object%20Reference))
  (bind (_x _y _z) (Math|Vector|BreakVector Vector))
  (bind _noiseweight (Variables|Default|GetNoiseWeight))
  (bind _returnvalue (Class|FastNoiseWrapper|GetNoise3D FastNoiseWrapper _x _y _z))
  (return (Math|Vector|MakeVector (+ _x (* _returnvalue _noiseweight)) (+ _y (* _returnvalue _noiseweight)) (* (Class|FastNoiseWrapper|GetNoise2D FastNoiseWrapper _x _y) _z))))