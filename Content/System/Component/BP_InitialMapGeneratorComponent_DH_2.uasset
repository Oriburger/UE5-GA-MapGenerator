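; Map generator component that lays platforms between the start and end locations of its owning BP_MapGeneratorBase.
; Generate steps along the straight line by the player's max speed, one second of travel per platform, storing the list in LastGenerateResult.
; An alternate CustomEvent keeps every PlatformIntervalSecond-th step, multiplies its height by randomly seeded 2D Perlin noise, and stores LastGenerateResultList.
; Both also add static mesh components to the owner for debugging.
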(event Custom|CustomEvent
  (bind _returnvalue (Game|GetPlayerCharacter 0))
  (bind _platformlist (Variables|Default|GetPlatformList))
  (bind _charactermovement (Variables|/Script/Engine.Character|GetCharacterMovement _returnvalue))
  (bind _returnvalue_2 (Class|MovementComponent|GetMaxSpeed _charactermovement))
  ;[0.9667 0.4177 1 1 33] 맵 생성 알고리즘 1 _ 권대현
  ;;[1 1 1] Get Reference
  (|CallParentFunction)
  (bind _asbp_map_generator_base (Utilities|Casting|CastToBP_MapGeneratorBase (Components|GetOwner)))
  ;;[1 1 1] Perlin Noise
  (bind _returnvalue_3 (Game|ConstructObjectfromClass "/Script/FastNoiseGenerator.FastNoiseWrapper"))
  (Class|FastNoiseWrapper|SetupFastNoise _returnvalue_3 "Perlin" (Math|Random|RandomInteger 9999) 0.01 "Quintic" "FBM" 3 2.0 0.5 0.45 "Euclidean" "CellValue")
  (for _index (range 0 (Math|Float|Ceil (/ (Math|Vector|Distance(Vector) (Variables|/Script/AnotherWorldStreet.MapGeneratorBase|GetStartLocation _asbp_map_generator_base) (Variables|/Script/AnotherWorldStreet.MapGeneratorBase|GetEndLocation _asbp_map_generator_base)) _returnvalue_2)))
    (if (== (Math|Integer|%(Integer) _index (Variables|Default|GetPlatformIntervalSecond)) 0)
      ;;[1 1 1] Platform 생성
      (bind _newvector (CallFunction|SetPerlinVector (Math|Interpolation|VInterptoConstant (Variables|/Script/AnotherWorldStreet.MapGeneratorBase|GetStartLocation _asbp_map_generator_base) (Variables|/Script/AnotherWorldStreet.MapGeneratorBase|GetEndLocation _asbp_map_generator_base) (Math|Conversions|ToFloat(Integer) _index) _returnvalue_2) _returnvalue_3))
      (Development|PrintString (Utilities|String|ToString(Vector) _newvector))
      (Utilities|Array|Add _platformlist (Utilities|Struct|MakePlatformInfoStruct "/Game/Asset/Platformer/Meshes/Pl_4m_Platform.Pl_4m_Platform" (Math|Transform|MakeTransform _newvector)))
      ;[1 1 1] 메시 생성(디버그)
      (bind _returnvalue_4 (Game|AddComponentbyClass _asbp_map_generator_base "/Script/Engine.StaticMeshComponent" false (Math|Transform|MakeTransform _newvector)))
      (Components|StaticMesh|SetStaticMesh _returnvalue_4 "/Game/Asset/Platformer/Meshes/Pl_8m_Platform.Pl_8m_Platform")))
  (Variables|Default|SetLastGenerateResultList (Utilities|Array|MakeArray (Utilities|Struct|MakeMapInfoStruct _platformlist 0 0.0))))

(event EventGenerate
  (bind _returnvalue (Game|GetPlayerCharacter 0))
  (bind _platformlist (Variables|Default|GetPlatformList))
  (bind _charactermovement (Variables|/Script/Engine.Character|GetCharacterMovement _returnvalue))
  (bind _returnvalue_2 (Class|MovementComponent|GetMaxSpeed _charactermovement))
  ;[0.9667 0.4177 1 1 33] 맵 생성 알고리즘 2 _ 권대현
  ;;[1 1 1] Get Reference
  (|CallParentFunction)
  (bind _asbp_map_generator_base (Utilities|Casting|CastToBP_MapGeneratorBase (Components|GetOwner)))
  (Utilities|Array|Add _platformlist (Utilities|Struct|MakePlatformInfoStruct "/Game/Asset/Platformer/Meshes/Pl_8m_Platform.Pl_8m_Platform" (Math|Conversions|ToTransform(Vector) (Variables|/Script/AnotherWorldStreet.MapGeneratorBase|GetStartLocation _asbp_map_generator_base))))
  (for _index (range 0 (Math|Float|Ceil (/ (Math|Vector|Distance(Vector) (Variables|/Script/AnotherWorldStreet.MapGeneratorBase|GetStartLocation _asbp_map_generator_base) (Variables|/Script/AnotherWorldStreet.MapGeneratorBase|GetEndLocation _asbp_map_generator_base)) _returnvalue_2)))
    (Utilities|Array|Add _platformlist (Utilities|Struct|MakePlatformInfoStruct "/Game/Asset/Platformer/Meshes/Pl_8m_Platform.Pl_8m_Platform" (Math|Transform|MakeTransform (Math|Interpolation|VInterptoConstant (Variables|/Script/AnotherWorldStreet.MapGeneratorBase|GetStartLocation _asbp_map_generator_base) (Variables|/Script/AnotherWorldStreet.MapGeneratorBase|GetEndLocation _asbp_map_generator_base) (Math|Conversions|ToFloat(Integer) _index) _returnvalue_2))))
    ;[1 1 1] 메시 생성(디버그)
    (bind _returnvalue_3 (Game|AddComponentbyClass _asbp_map_generator_base "/Script/Engine.StaticMeshComponent" false (Math|Transform|MakeTransform (Math|Interpolation|VInterptoConstant (Variables|/Script/AnotherWorldStreet.MapGeneratorBase|GetStartLocation _asbp_map_generator_base) (Variables|/Script/AnotherWorldStreet.MapGeneratorBase|GetEndLocation _asbp_map_generator_base) (Math|Conversions|ToFloat(Integer) _index) _returnvalue_2))))
    (Components|StaticMesh|SetStaticMesh _returnvalue_3 "/Game/Asset/Platformer/Meshes/Pl_8m_Platform.Pl_8m_Platform"))
  (Variables|Default|SetLastGenerateResult (Utilities|Struct|MakeMapInfoStruct _platformlist 0 0.0)) ; 지우면 안되빈다
)

(fn SetPerlinVector
  (params (Vector :type Vector) (FastNoiseWrapper :type Fast%20Noise%20Wrapper%20Object%20Reference))
  (bind (_x _y _z) (Math|Vector|BreakVector Vector))
  (return (Math|Vector|MakeVector _x _y (* (Class|FastNoiseWrapper|GetNoise2D FastNoiseWrapper _x _y) _z))))