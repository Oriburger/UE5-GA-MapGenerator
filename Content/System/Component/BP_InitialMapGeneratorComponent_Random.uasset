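; Map generator component that builds an initial population of random platform maps for its BP_MapGeneratorBase owner.
; Generate loops up to the owner's PopulationSize, adding each RandomlyGenerate result to LastGenerateResultList.
; Each map gets a few hundred platforms with random meshes from the owner's list at random positions within MapSize.
; The middle-index platform is pinned to the map's center.
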(event EventGenerate
  ;[0.6037 0.4074 1 1 33] 맵 생성 알고리즘 _ 랜덤
  (|CallParentFunction)
  (bind _asbp_map_generator_base (Utilities|Casting|CastToBP_MapGeneratorBase (Components|GetOwner)))
  (bind _output_get (Variables|Default|SetAs%20BP%20Map%20Generator%20Base _asbp_map_generator_base))
  (if (< (Variables|Default|GetIdx) (Variables|/Script/AnotherWorldStreet.MapGeneratorBase|GetPopulationSize _output_get)) :!label _label
    ;;[1 1 1] 이곳에 구현
    (bind _result (CallFunction|RandomlyGenerate))
    (Utilities|Array|Add (Variables|Default|GetLastGenerateResultList) _result)
    (Math|Integer|IncrementInt (Variables|Default|GetIdx)
      (:%20%20
        (goto _label)))))

(fn RandomlyGenerate
  (bind _as_bp_map_generator_base (Variables|Default|GetAs%20BP%20Map%20Generator%20Base))
  (bind _mapsize (Variables|/Script/AnotherWorldStreet.MapGeneratorBase|GetMapSize _as_bp_map_generator_base))
  (bind _output_get (LocalVariables|Setrange (Math|Random|RandomIntegerinRange 250 500)))
  (for _index (range 0 _output_get)
    (Utilities|Array|Add (.platforminfolist (LocalVariables|GetresultMap)) (Utilities|Struct|MakePlatformInfoStruct (.OutItem (Utilities|Array|Random (Variables|/Script/AnotherWorldStreet.MapGeneratorBase|GetPlatformMeshList _as_bp_map_generator_base))) (Math|Transform|MakeTransform (Math|Vector|SelectVector (/ (Variables|/Script/AnotherWorldStreet.MapGeneratorBase|GetMapSize _as_bp_map_generator_base) 2.0) (Math|Vector|MakeVector (Math|Random|RandomFloatinRange 0.0 (.x _mapsize)) (Math|Random|RandomFloatinRange 0.0 (.y _mapsize)) (Math|Random|RandomFloatinRange 0.0 (.z _mapsize))) (== _index (/ _output_get 2))) "0, 0, 0" "1.000000,1.000000,1.000000"))))
  (return (LocalVariables|GetresultMap)))