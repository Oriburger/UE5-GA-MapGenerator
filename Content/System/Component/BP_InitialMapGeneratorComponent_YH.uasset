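; Map generator component that lays a curved trail of 4m platforms between the owning BP_MapGeneratorBase's start and end locations.
; Generate samples a quadratic Bézier curve bent by a random control point within fixed absolute coordinate ranges.
; Each sampled point becomes a platform transform with random yaw, stored in LastGenerateResult.
; The curve function only produces points when given a control-point count of one.
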(event EventBeginPlay
  (bind _asbp_map_generator_base (Utilities|Casting|CastToBP_MapGeneratorBase (Components|GetOwner)))
  (Variables|Default|SetAs%20BP%20Map%20Generator%20Base _asbp_map_generator_base))

(event EventGenerate
  ;[0.6037 0.4074 1 1 33] 맵 생성 알고리즘 _ 황유호
  (|CallParentFunction)
  (bind _as_bp_map_generator_base (Variables|Default|GetAs%20BP%20Map%20Generator%20Base)
    (:then
      (CallFunction|GenBezierCurve (Math|Conversions|ToTransform(Vector) (Variables|/Script/AnotherWorldStreet.MapGeneratorBase|GetStartLocation _as_bp_map_generator_base)) (Math|Conversions|ToTransform(Vector) (Variables|/Script/AnotherWorldStreet.MapGeneratorBase|GetEndLocation _as_bp_map_generator_base)) 14 1)
      (for _array_element (Variables|Default|GetCurvePoints)
        (Utilities|Array|Add (Variables|Default|GetPoint3D) (Utilities|Struct|MakePoint3D (.x (Utilities|Struct|BreakPoint3D _array_element)) (.y (Utilities|Struct|BreakPoint3D _array_element)) (.z (Utilities|Struct|BreakPoint3D _array_element)))))
      (for _array_element_2 (Variables|Default|GetPoint3D)
        (Utilities|Array|Add (Variables|Default|GetPlatform_Info) (Utilities|Struct|MakePlatformInfoStruct "/Game/Asset/Platformer/Meshes/Pl_4m_Platform.Pl_4m_Platform" (Math|Transform|MakeTransform (Math|Vector|MakeVector (.x (Utilities|Struct|BreakPoint3D _array_element_2)) (.y (Utilities|Struct|BreakPoint3D _array_element_2)) (.z (Utilities|Struct|BreakPoint3D _array_element_2))) (Math|Rotator|MakeRotator 0.0 0.0 (.yaw (Math|Random|RandomRotator false)))))))
      (Variables|Default|SetLastGenerateResult (Utilities|Struct|MakeMapInfoStruct (Variables|Default|GetPlatform_Info) 0 0.0)) ; 지우면 안되빈다
    )
    (:else)))

(fn GenRandomControlPoint
  (bind _output_get (LocalVariables|SetPoint3D_local (Utilities|Struct|MakePoint3D (Math|Random|RandomFloatinRange 5e+03 1e+04) (Math|Random|RandomFloatinRange 5e+03 1e+04) (Math|Random|RandomFloatinRange 1.5e+03 2.5e+03))))
  (return _output_get))

(fn GenBezierCurve
  (params (StartPoint :type Transform) (EndPoint :type Transform) (numPoints :type Integer) (numContorlPoints :type Integer))
  (bind _location (Math|Transform|BreakTransform StartPoint))
  (bind _location_2 (Math|Transform|BreakTransform EndPoint))
  (bind _controlpoint (LocalVariables|GetControlPoint))
  (bind _output (Utilities|Array|Get(acopy) _controlpoint))
  (bind (_x _y _z) (Utilities|Struct|BreakPoint3D _output))
  (for _index (range 0 numContorlPoints)
    (bind _point_x_y_z_ (CallFunction|GenRandomControlPoint))
    (Utilities|Array|Add (LocalVariables|GetControlPoint) _point_x_y_z_))
  (if (== numContorlPoints 1)
    (for _index_2 (range 0 numPoints)
      (bind _output_get (LocalVariables|Sett (/ (Math|Conversions|ToFloat(Integer) _index_2) (- numPoints 1))))
      (bind _output_get_2 (LocalVariables|SetoneMinusT (- 1.0 _output_get)))
      (LocalVariables|SettSquared (Math|Float|Square _output_get))
      (LocalVariables|SetoneMinusTSquared (Math|Float|Square _output_get_2))
      (Utilities|Array|Add (Variables|Default|GetCurvePoints) (Utilities|Struct|MakePoint3D (+ (* (.x _location_2) (LocalVariables|GettSquared)) (+ (* 2.0 (* _x (* (LocalVariables|GetoneMinusT) (LocalVariables|Gett)))) (* (.x _location) (LocalVariables|GetoneMinusTSquared)))) (+ (* (.y _location_2) (LocalVariables|GettSquared)) (+ (* 2.0 (* _y (* (LocalVariables|GetoneMinusT) (LocalVariables|Gett)))) (* (.y _location) (LocalVariables|GetoneMinusTSquared)))) (+ (* (.z _location_2) (LocalVariables|GettSquared)) (+ (* 2.0 (* _z (* (LocalVariables|GetoneMinusT) (LocalVariables|Gett)))) (* (.z _location) (LocalVariables|GetoneMinusTSquared)))))))))